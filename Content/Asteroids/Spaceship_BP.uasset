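; Player spaceship Blueprint for an Asteroids game, steered by physics and able to shoot.
; Rotate and MoveForward axes apply torque and forward force to the ship mesh as acceleration changes, while Shoot spawns a Bullet_BP at the spawn point with a laser sound.
; Overlapping an asteroid kills it and calls ReduceHealth, which hides health indicator components and, at zero, destroys the ship and reloads Asteroids_Level.
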(event `self.CollisionSpaceship.OnComponentBeginOverlap`
  (params (OverlappedComponent :type "PrimitiveComponent Object Reference") (OtherActor :type "Actor Object Reference") (OtherComp :type "PrimitiveComponent Object Reference") (OtherBodyIndex :type Integer) (bFromSweep :type Boolean) (SweepResult :type "HitResult Structure (by ref)"))
  (bind _asasteroids_base_bp (cast `/Game/Asteroids/AsteroidsBase_BP` OtherActor))
  (`self.ReduceHealth`)
  (`/Game/Asteroids/AsteroidsBase_BP.Death` _asasteroids_base_bp))

(event `InputAxis|Rotate`
  (params (AxisValue :type "Float (single-precision)"))
  (`PrimitiveComponent.AddTorqueInDegrees` (`self.Spaceship_SM`) (`KismetMathLibrary.MakeVector` 0.0 0.0 (* AxisValue (`self.TorqueMultiplier`))) "None" true))

(event `InputAxis|MoveForward`
  (params (AxisValue :type "Float (single-precision)"))
  (bind _spaceship_sm (`self.Spaceship_SM`))
  (`PrimitiveComponent.AddForce` _spaceship_sm (* (* AxisValue (`self.ForwardSpeedMultiplier`)) (`SceneComponent.GetForwardVector` _spaceship_sm)) "None" true))

(event `InputAction|Shoot`
  (params (Key :type "Key Structure"))
  (:`Pressed`
    (`|SpawnActorFromClass` "/Game/Asteroids/Bullet_BP.Bullet_BP_C" (`SceneComponent.K2_GetComponentToWorld` (`self.BulletSpawnPoint`)) "AdjustIfPossibleButAlwaysSpawn" "MultiplyWithRoot" null null)
    (`GameplayStatics.PlaySound2D` "/Game/Asteroids/Sounds/Laser_Shoot31.Laser_Shoot31" 1.0 1.0 0.0 null null)))

(fn `ReduceHealth`
  (bind _output_get (set `self.Health` (- (`self.Health`) 1)))
  (switch `int` _output_get
    (:`0`
      (`self.K2_DestroyActor`)
      (`GameplayStatics.OpenLevel` "Asteroids_Level"))
    (:`1`
      (`SceneComponent.SetVisibility` (`self.Health1`) false false))
    (:`2`
      (`SceneComponent.SetVisibility` (`self.Health2`) false false))
    (:`3`
      (`SceneComponent.SetVisibility` (`self.Health0`) true false)
      (`SceneComponent.SetVisibility` (`self.Health1`) true false)
      (`SceneComponent.SetVisibility` (`self.Health2`) true false))))

(fn `UserConstructionScript`)